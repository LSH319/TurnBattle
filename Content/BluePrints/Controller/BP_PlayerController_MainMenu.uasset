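; Main menu player controller that sets up the camera and UI when play begins.
; It views through a random camera tagged "Start", adds the primary layout widget to the viewport, and shows the cursor with game-and-UI input.
; It pushes an OK caution screen noting the portfolio project, plus a soft-referenced Press Any Key widget resolved by gameplay tag onto the GameHud stack.
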(event `self.ReceiveBeginPlay`
  (bind _outactors (`GameplayStatics.GetAllActorsOfClassWithTag` "/Script/Engine.CameraActor" "Start"))
  (`self.SetViewTargetWithBlend` (`KismetArrayLibrary.Array_Random` _outactors))
  (bind _returnvalue (`|CreateWidget` "/Game/UI/Widget/WBP_PrimaryLayoutWidget.WBP_PrimaryLayoutWidget_C" self))
  (`UserWidget.AddToViewport` _returnvalue 0)
  (`WidgetBlueprintLibrary.SetInputMode_GameAndUIEx` self null)
  (set `self.bShowMouseCursor` true)
  (`LshPF_PushConfirmScreen.PushConfirmScreen` "/Game/UI/Widget/ConfirmScreen/WBP_FW_ConfirmScreen_Base.WBP_FW_ConfirmScreen_Base_C" "Ok" "Caution" "This Project is Just My Portfolio"
    (:`then`
      (`LshPF_PushSoftWidget.PushSoftWidget` self (`LshPF_FunctionLibrary.GetSoftFocusableWidgetBaseClassByTag` (struct :`TagName` "LshPF.Widget.PressAnyKey")) (struct :`TagName` "LshPF.WidgetStack.GameHud") false))))

(fn `UserConstructionScript`
  (`parent.UserConstructionScript`))