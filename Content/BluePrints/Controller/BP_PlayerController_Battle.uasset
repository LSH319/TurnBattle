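; BP_PlayerController_Battle is the player controller for battle, setting up the camera, UI and battle menu input.
; On BeginPlay it blends view to a random CameraActor tagged "Start", adds the primary layout widget, and enables Game-and-UI input with a visible cursor.
; The Item and Skill Enhanced Input actions each push their battle widget as a soft class onto the GameHud tagged widget stack.
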(event `self.ReceiveBeginPlay`
  (bind _outactors (`GameplayStatics.GetAllActorsOfClassWithTag` "/Script/Engine.CameraActor" "Start"))
  (`self.SetViewTargetWithBlend` (`KismetArrayLibrary.Array_Random` _outactors))
  (bind _returnvalue (`|CreateWidget` "/Game/UI/Widget/WBP_PrimaryLayoutWidget.WBP_PrimaryLayoutWidget_C" self))
  (`UserWidget.AddToViewport` _returnvalue 0)
  (`WidgetBlueprintLibrary.SetInputMode_GameAndUIEx` self null)
  (set `self.bShowMouseCursor` true))

(event `EnhancedInput|/Game/Input/IA/Battle/IA_Battle_Item`
  (params (ActionValue :type Boolean) (ElapsedSeconds :type "Float (double-precision)") (TriggeredSeconds :type "Float (double-precision)") (InputAction :type "InputAction Object Reference" :default "/Game/Input/IA/Battle/IA_Battle_Item.IA_Battle_Item"))
  (:`Started`
    (`LshPF_PushSoftWidget.PushSoftWidget` null "/Game/UI/Widget/Battle/WBP_FW_Battle_Item.WBP_FW_Battle_Item_C" (struct :`TagName` "LshPF.WidgetStack.GameHud"))))

(event `EnhancedInput|/Game/Input/IA/Battle/IA_Battle_Skill`
  (params (ActionValue :type Boolean) (ElapsedSeconds :type "Float (double-precision)") (TriggeredSeconds :type "Float (double-precision)") (InputAction :type "InputAction Object Reference" :default "/Game/Input/IA/Battle/IA_Battle_Skill.IA_Battle_Skill"))
  (:`Started`
    (`LshPF_PushSoftWidget.PushSoftWidget` null "/Game/UI/Widget/Battle/WBP_FW_Battle_Skill.WBP_FW_Battle_Skill_C" (struct :`TagName` "LshPF.WidgetStack.GameHud"))))

(fn `UserConstructionScript`)