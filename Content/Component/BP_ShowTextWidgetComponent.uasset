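; Widget component that briefly shows an applied value as text, distinguishing damage from non-damage values by color.
; SetApplyText casts its user widget to WBP_ApplyValueText, sets the text, and colors it white for damage or green otherwise.
; After a short delay the component destroys itself, so each instance serves as a one-shot popup.
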(event `self.SetApplyText`
  (params (Text :type String) (IsDamage :type Boolean))
  (bind _aswbp_apply_value_text (cast `/Game/UI/Widget/Battle/WBP_ApplyValueText` (`self.GetUserWidgetObject`)))
  (bind _applyvaluetext (`/Game/UI/Widget/Battle/WBP_ApplyValueText.ApplyValueText` _aswbp_apply_value_text))
  (`TextBlock.SetText` _applyvaluetext (`KismetTextLibrary.Conv_StringToText` Text))
  (`TextBlock.SetColorAndOpacity` _applyvaluetext (select `bool` IsDamage :`false` (make `SlateColor` (struct :`G` 1.0 :`A` 1.0)) :`true` (make `SlateColor` (struct :`R` 1.0 :`G` 1.0 :`B` 1.0 :`A` 1.0))))
  (`KismetSystemLibrary.Delay` 0.5)
  (`self.K2_DestroyComponent`))